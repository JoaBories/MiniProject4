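; BP_NPC2 is an enemy NPC with pistols that damages the player through a line trace.
; PrepareAttack swaps the mesh material as a tell; Attack traces, damages the player if hit, then plays a timeline pistol animation before restoring the material.
; Hits subtract health and briefly zero walk speed as a stun.
; Death spawns an explosion, destroys the actor and makes two random rolls for medkit or shotgun shell drops.
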(event Custom|Hit
  (params (StunTime :type Float%20%28double-precision%29) (Damage :type Float%20%28double-precision%29))
  (bind _charactermovement (Variables|Character|GetCharacterMovement))
  (bind _output_get (Variables|Default|SetHp (- (Variables|Default|GetHp) Damage)))
  (if (> _output_get 0.0)
    ;[1 1 1] Stun
    (Variables|/Script/Engine.CharacterMovementComponent|SetMaxWalkSpeed _charactermovement 0.0)
    (Utilities|FlowControl|Delay StunTime)
    (Variables|/Script/Engine.CharacterMovementComponent|SetMaxWalkSpeed _charactermovement (Variables|Default|GetMax%20Walk%20Speed))
    (else
      (Gameplay|Die))))

(event Custom|PrepareAttack
  (Rendering|Material|SetMaterial (Variables|Default|GetStaticMesh) 0 (Variables|Default|GetAttackMat)))

(event Custom|Attack
  (bind _returnvalue (Game|Player|GetPlayerPawn 0))
  (Utilities|FlowControl|Sequence
    (:then_0
      (bind (_returnvalue_2 _hitactor) (|LineTrace))
      (if _returnvalue_2
        (|TellPlayerHit (== _hitactor _returnvalue) _returnvalue)))
    (:then_1
      (|PistolAnim
        (:Finished
          (Rendering|Material|SetMaterial (Variables|Default|GetStaticMesh) 0 (Variables|Default|GetNormalMat)))))))

(event EventBeginPlay
  (Variables|Default|SetMax%20Walk%20Speed (Variables|/Script/Engine.CharacterMovementComponent|GetMaxWalkSpeed (Variables|Character|GetCharacterMovement)))
  (Variables|Default|SetHp (Variables|Default|GetMaxHP)))

(fn ConstructionScript)