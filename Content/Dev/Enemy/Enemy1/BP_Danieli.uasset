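; BP_Danieli is a pistol-wielding enemy that shoots the player with a hitscan attack.
; PrepareAttack swaps in an attack material and turns it toward the player on a timeline; Attack line-traces past Danieli and Franchesca actors, damages the player, and plays tracer effects and pistol animation.
; Hit subtracts health, ignoring StunTime; death triggers an explosion, a random medkit or shotgun shell drop, and updates the game mode's enemy count.
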(event Custom|Hit
  (params (StunTime :type Float%20%28double-precision%29) (Damage :type Float%20%28double-precision%29))
  (bind _output_get (Variables|Default|SetHp (- (Variables|Default|GetHp) Damage)))
  (if (not (> _output_get 0.0))
    (Gameplay|Die)))

(event Custom|PrepareAttack
  (Rendering|Material|SetMaterial (Variables|Default|GetStaticMesh) 1 (Variables|Default|GetAttackMat))
  (bind _newtrack_0 (Timeline|AimPlayer PlayFromStart)
    (:Update
      (Transformation|SetActorRotation (Math|Rotator|Lerp(Rotator) (Transformation|GetActorRotation) (Math|Rotator|MakeRotationfromAxes (- (Transformation|GetActorLocation (Game|Player|GetPlayerPawn 0)) (Transformation|GetActorLocation)) "0, 0, 0" "0, 0, 0") _newtrack_0 true)))))

(event Custom|Attack
  (bind _returnvalue (Game|Player|GetPlayerPawn 0))
  (Utilities|FlowControl|Sequence
    (:then_0
      (bind _outactors (Actor|GetAllActorsOfClass "BP_Danieli_C"))
      (bind _output_get (Variables|Default|SetIgnoreActors _outactors))
      (bind _outactors_2 (Actor|GetAllActorsOfClass "/Game/Dev/Enemy/Enemy2/BP_Franchesca.BP_Franchesca_C"))
      (Utilities|Array|AppendArray _output_get _outactors_2)
      (bind (_returnvalue_2 _impactpoint _hitactor) (|LineTrace (Variables|Default|GetIgnoreActors)))
      (if _returnvalue_2
        (|TellPlayerHit (== _hitactor _returnvalue) _returnvalue)))
    (:then_1
      (|PlayVFX (== _hitactor _returnvalue) _impactpoint))
    (:then_2
      (Rendering|Material|SetMaterial (Variables|Default|GetStaticMesh) 1 (Variables|Default|GetNormalMat)))
    (:then_3
      (|PistolAnim))))

(event EventBeginPlay
  (Variables|Default|SetMax%20Walk%20Speed (Variables|/Script/Engine.CharacterMovementComponent|GetMaxWalkSpeed (Variables|Character|GetCharacterMovement)))
  (Variables|Default|SetHp (Variables|Default|GetMaxHP)))

(fn ConstructionScript)