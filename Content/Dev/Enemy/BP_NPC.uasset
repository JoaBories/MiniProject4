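; BP_NPC is a pistol-wielding enemy that shoots the player and drops loot on death.
; Hit subtracts health, stuns survivors by zeroing walk speed, or triggers an explosion, a random medic box or shotgun shell drop, and destruction.
; PrepareAttack swaps in a warning material and turns toward the player on a timeline.
; Attack line-traces to damage the player, restores the material, and plays Niagara shot effects and a pistol animation.
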(event Custom|Hit
  (params (StunTime :type Float%20%28double-precision%29) (Damage :type Float%20%28double-precision%29))
  (bind _returnvalue (Transformation|GetActorTransform))
  (bind _charactermovement (Variables|Character|GetCharacterMovement))
  (bind (_location _rotation) (Math|Transform|BreakTransform _returnvalue))
  (bind _output_get (Variables|Default|SetHp (- (Variables|Default|GetHp) Damage)))
  (if (> _output_get 0.0)
    ;[1 1 1] Stun
    (Variables|/Script/Engine.CharacterMovementComponent|SetMaxWalkSpeed _charactermovement 0.0)
    (Utilities|FlowControl|Delay StunTime)
    (Variables|/Script/Engine.CharacterMovementComponent|SetMaxWalkSpeed _charactermovement (Variables|Default|GetMax%20Walk%20Speed))
    (else
      (Utilities|FlowControl|Sequence
        (:then_0
          (Niagara|SpawnSystematLocation "/Game/NiagaraSystem/NS_Explosion.NS_Explosion" (Transformation|GetActorLocation)))
        (:then_1
          (switch int (Math|Random|RandomInteger 2)
            (:0
              (bind _returnvalue_2 (Game|SpawnActorfromClass "/Game/Dev/BP_MedicBox.BP_MedicBox_C" _returnvalue "Undefined" "MultiplyWithRoot" 0 0))
              (Niagara|SpawnSystematLocation "/Game/NiagaraSystem/NS_DropMedic.NS_DropMedic" _location _rotation))
            (:1
              (bind _returnvalue_3 (Game|SpawnActorfromClass "/Game/Dev/BP_ShotgunShell.BP_ShotgunShell_C" _returnvalue "Undefined" "MultiplyWithRoot" 0 0 :!label _label))
              (Niagara|SpawnSystematLocation "/Game/NiagaraSystem/NS_DropShell.NS_DropShell" _location _rotation))
            (:2
              (goto _label))))
        (:then_2
          (Actor|DestroyActor))))))

(event Custom|PrepareAttack
  (Rendering|Material|SetMaterial (Variables|Default|GetStaticMesh) 1 (Variables|Default|GetAttackMat))
  (bind _newtrack_0 (Timeline|AimPlayer PlayFromStart)
    (:Update
      (Transformation|SetActorRotation (Math|Rotator|Lerp(Rotator) (Transformation|GetActorRotation) (Math|Rotator|MakeRotationfromAxes (- (Transformation|GetActorLocation (Game|Player|GetPlayerPawn 0)) (Transformation|GetActorLocation)) "0, 0, 0" "0, 0, 0") _newtrack_0 true)))))

(event Custom|Attack
  (bind _returnvalue (Game|Player|GetPlayerPawn 0))
  (bind (_returnvalue_2 _returnvalue2 _array) (|CollapseGraph))
  (bind _pistolcanon (Variables|Default|GetPistolCanon))
  (bind _returnvalue_3 (Transformation|GetWorldLocation _pistolcanon))
  (Utilities|FlowControl|Sequence
    (:then_0
      (bind (_outhit _returnvalue_4) (Collision|LineTraceForObjects _returnvalue_2 _returnvalue2 _array false 0 "ForDuration"))
      (Rendering|Material|SetMaterial (Variables|Default|GetStaticMesh) 1 (Variables|Default|GetNormalMat))
      (if _returnvalue_4
        (if (== (.HitActor (Collision|BreakHitResult _outhit)) _returnvalue)
          (bind _asbp_fps_character (Utilities|Casting|CastToBP_FpsCharacter _returnvalue))
          (Default|TakeDamage _asbp_fps_character (Variables|Default|GetDamage)))))
    (:then_1
      (Niagara|SpawnSystematLocation "/Game/NiagaraSystem/NS_MuzzleFlash.NS_MuzzleFlash" _returnvalue_3 (Transformation|GetWorldRotation _pistolcanon))
      (if (== (.HitActor (Collision|BreakHitResult _outhit)) _returnvalue)
        (bind _returnvalue_5 (Niagara|SpawnSystematLocation "/Game/NiagaraSystem/NS_BulletTraceEnemyHit.NS_BulletTraceEnemyHit" "0, 0, 0"))
        (Niagara|SetNiagaraVariable(Vector3) _returnvalue_5 "CanonPos" "0, 0, 0")
        (else
          (bind _returnvalue_6 (Niagara|SpawnSystematLocation "/Game/NiagaraSystem/NS_ShotgunBulletTrace.NS_ShotgunBulletTrace" (.ImpactPoint (Collision|BreakHitResult _outhit))))
          (Niagara|SetNiagaraVariable(Vector3) _returnvalue_6 "CanonPos" _returnvalue_3))))
    (:then_2
      (bind _newtrack_0 (Timeline|Anim PlayFromStart)
        (:Update
          (Transformation|SetRelativeRotation (Variables|Default|GetPistol) (Math|Rotator|MakeRotator 0.0 _newtrack_0 0.0) false false))))))

(event EventBeginPlay
  (Variables|Default|SetMax%20Walk%20Speed (Variables|/Script/Engine.CharacterMovementComponent|GetMaxWalkSpeed (Variables|Character|GetCharacterMovement)))
  (Variables|Default|SetHp 1.0))

(fn ConstructionScript)