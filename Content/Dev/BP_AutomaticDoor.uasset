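; BP_AutomaticDoor is a door actor that rises vertically when the player approaches and stays open.
; BeginPlay caches the starting world Z, and a Sphere overlap by player pawn 0 destroys the trigger, making the opening one-shot.
; The Opening timeline then lerps the actor's Z from that start to TopPos, an absolute world height, keeping X and Y unchanged.
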(event OnComponentBeginOverlap(Sphere)
  (params (OverlappedComponent :type Primitive%20Component%20Object%20Reference) (OtherActor :type Actor%20Object%20Reference) (OtherComp :type Primitive%20Component%20Object%20Reference) (OtherBodyIndex :type Integer) (bFromSweep :type Boolean) (SweepResult :type Hit%20Result%20Structure%20%28by%20ref%29))
  (bind _returnvalue (Transformation|GetActorLocation))
  (if (== OtherActor (Game|Player|GetPlayerPawn 0))
    (Components|DestroyComponent (Variables|Default|GetSphere))
    (bind _opening (Timeline|opening PlayFromStart)
      (:Update
        (Transformation|SetActorLocation (Math|Vector|MakeVector (.x _returnvalue) (.y _returnvalue) (Math|Float|Lerp (Variables|Default|GetInitialPos) (Variables|Default|GetTopPos) _opening)) false false)))))

(event EventBeginPlay
  (Variables|Default|SetInitialPos (.z (Transformation|GetActorLocation))))

(fn ConstructionScript)